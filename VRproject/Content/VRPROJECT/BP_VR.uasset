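; VR player pawn handling teleport movement, camera turning, object grabbing, widget clicks and a simple inventory.
; While right trigger or left mouse is held, a projectile arc from the camera finds flat ground, projects it to the navmesh and draws a debug cylinder; release teleports.
; Left trigger toggles grabbing through IGrapped; right grip sends InteractMessage to an overlapped actor.
; The spline arc display is unfinished: SplineUpdate's body never runs.
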(event EventBeginPlay
  (Class|HeadMountedDisplayFunctionLibrary|SetTrackingOrigin "Eye"))

(event Collision|EventActorBeginOverlap
  (params (OtherActor :type Actor%20Object%20Reference)))

(event EventTick
  (params (DeltaSeconds :type Float%20%28single-precision%29))
  (bind _camera (Variables|Default|GetCamera))
  ;[1 1 1] 텔레포트 및 이동기
  (if (Variables|Default|GetfindTeleport)
    (Teleport|ClearSpline)
    (Teleport|LocationDetect (Transformation|GetWorldLocation _camera) (Math|Vector|GetForwardVector _camera))))

(event EventAddInventory
  (params (item :type String))
  ;[1 1 1] 인벤토리
  (Utilities|Array|Add (Variables|Default|GetInventory) item))

(event Input|AxisEvents|InputAxisTurn
  (params (AxisValue :type Float%20%28single-precision%29))
  ;[1 1 1] 화면회전
  (Transformation|AddRelativeRotation (Variables|Default|GetCamera) (Math|Rotator|MakeRotator 0.0 0.0 AxisValue) false false))

(event Input|AxisEvents|InputAxisUpdown
  (params (AxisValue :type Float%20%28single-precision%29))
  ;[1 1 1] 화면회전
  (Transformation|AddRelativeRotation (Variables|Default|GetCamera) (Math|Rotator|MakeRotator 0.0 AxisValue 0.0) false false))

(event Input|MouseEvents|LeftMouseButton
  (params (Key :type Key%20Structure))
  (bind _scene (Variables|Default|GetScene))
  (bind _camera (Variables|Default|GetCamera))
  (bind _telelocation (Variables|Default|GetTeleLocation))
  (bind (_x _y) (Math|Vector|BreakVector _telelocation))
  ;[1 1 1] 텔레포트 및 이동기
  (:Pressed
    (Teleport|LocationDetect (Transformation|GetWorldLocation _camera) (Math|Vector|GetForwardVector _camera)))
  (:Released
    (if (Variables|Default|GetCanTeleport)
      (Transformation|SetWorldLocation _scene (Math|Vector|MakeVector _x _y (.Z (Math|Vector|BreakVector (Transformation|GetWorldLocation _scene)))) false true))))

(event Input|KeyboardEvents|MotionControllerLeftTrigger
  (params (Key :type Key%20Structure))
  ;[1 1 1] 물체를 던지는 것
  (:Pressed
    ;;[1 1 1] 한번클릭으로 잡고 다시클릭으로 놓고
    (if (Variables|Default|GetactGrab)
      (CallFunction|Release)
      (else
        (CallFunction|Grab)))))

(event Input|KeyboardEvents|MotionControllerLeftShoulder
  (params (Key :type Key%20Structure))
  (bind _widgetinteraction (Variables|Default|GetWidgetInteraction))
  ;[1 1 1] 텔레포트 및 이동기
  (:Pressed
    (Class|WidgetInteractionComponent|PressPointerKey _widgetinteraction "RightMouseButton"))
  (:Released
    (Class|WidgetInteractionComponent|ReleasePointerKey _widgetinteraction "RightMouseButton")))

(event Input|KeyboardEvents|MotionControllerRightTrigger
  (params (Key :type Key%20Structure))
  ;[1 1 1] 텔레포트 및 이동기
  (:Pressed
    (Variables|Default|SetfindTeleport true))
  (:Released
    (Variables|Default|SetfindTeleport false)
    (Teleport|ClearSpline)
    (if (Variables|Default|GetCanTeleport)
      (Transformation|SetWorldLocation (Variables|Default|GetScene) (Variables|Default|GetTeleLocation) false true))))

(event Input|MouseEvents|LeftMouseButton
  (params (Key :type Key%20Structure))
  ;[1 1 1] 텔레포트 및 이동기
  (:Pressed
    (Variables|Default|SetfindTeleport true))
  (:Released
    (Variables|Default|SetfindTeleport false)
    (Teleport|ClearSpline)
    (if (Variables|Default|GetCanTeleport)
      (Transformation|SetWorldLocation (Variables|Default|GetScene) (Variables|Default|GetTeleLocation) false true))))

(event Input|KeyboardEvents|MotionControllerRightGrip1
  (params (Key :type Key%20Structure))
  ;[1 1 1] 물체잡기
  (:Pressed
    (Class|InteractableInterface|Interact(Message) (Utilities|Array|Get(acopy) (Collision|GetOverlappingActors (Variables|Default|GetR_Sphere) "/Game/VRPROJECT/baseinteractable.baseinteractable_C" :!class /Script/Engine.PrimitiveComponent)) (Variables|Default|GetR_MotionController))))

(fn ConstructionScript)

(fn LocationDetect
  (params (CtrlLocation :type Vector) (CtrlForward :type Vector))
  (bind (_outhit _outpathpositions) (Class|GameplayStatics|BlueprintPredictProjectilePathbyObjectType CtrlLocation (* CtrlForward 1e+03) true 0.0 (Utilities|Array|MakeArray "ObjectTypeQuery1") false 0 "None"))
  (if (> (Math|Vector|DotProduct (.Normal (Collision|BreakHitResult _outhit)) "0, 0,1.000000") 0.9)
    (bind _output_get (Variables|Default|SetCanTeleport (> (Math|Vector|DotProduct (.Normal (Collision|BreakHitResult _outhit)) "0, 0,1.000000") 0.9)))
    (Teleport|SplineUpdate _output_get _outpathpositions)
    (bind _output_get_2 (Variables|Default|SetTeleLocation (.ProjectedLocation (AI|Navigation|ProjectPointtoNavigation (.Location (Collision|BreakHitResult _outhit)) 0 0 "0, 0, 0"))))
    (Class|KismetSystemLibrary|DrawDebugCylinder _output_get_2 (+ _output_get_2 (* (.Normal (Collision|BreakHitResult _outhit)) 2e+01)) 4e+01 25 "(R=0.355736,G=0.250000,B=0.750000,A=1.000000)" 0.0 1.5)))

(fn SplineUpdate
  (params (canTeleport :type Boolean) (LocationVectors :type Array%20of%20Vectors)))

(fn ClearSpline
  (bind _splinemeshes (Variables|Default|GetSplineMeshes))
  ;[1 1 1] 이동지역선택 잘못했을때 위치설정 초기화주는 기능
  (Components|DestroyComponent _splinemeshes)
  (Utilities|Array|Clear _splinemeshes)
  (Spline|ClearSplinePoints (Variables|Default|GetSpline) true))

(fn Grab
  (Variables|Default|SetactGrab true)
  (bind _neargrab (CallFunction|Neargrab))
  (Utilities|IsValid _neargrab
    (:Is%20Valid
      (bind _output_get (Variables|Default|SetAttachedActor _neargrab))
      (Class|IGrapped|Grap(Message) _output_get (Variables|Default|GetL_MotionController)))))

(fn Neargrab
  ;[1 1 1] 모션컨트롤러로 그래핑하는것
  (for _array_element (Collision|GetOverlappingActors (Variables|Default|GetL_Sphere) 0 :!class /Script/Engine.PrimitiveComponent)
    (if (Utilities|DoesObjectImplementInterface _array_element "/Game/VRPROJECT/IGrapped.IGrapped_C")
      (if (< (Math|Vector|VectorLength (- (Transformation|GetActorLocation _array_element) (Transformation|GetWorldLocation (Variables|Default|GetL_Sphere)))) 1e+03)
        (Variables|Default|SetnearActor _array_element))))
  (return (Variables|Default|GetnearActor)))

(fn Release
  (Variables|Default|SetactGrab false)
  (Utilities|IsValid (Variables|Default|GetAttachedActor)
    (:Is%20Valid
      (if true
        (Class|IGrapped|Release(Message) (Variables|Default|GetAttachedActor))
        ;[1 1 1] 널값할당
        (Variables|Default|SetAttachedActor 0)))))

(fn CheckInventory
  (params (item :type String))
  (return (Utilities|Array|ContainsItem (Variables|Default|GetInventory) item)))