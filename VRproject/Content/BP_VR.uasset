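; BP_VR is a camera actor with mouse-driven look and point-and-click teleport movement.
; Turn and LookUp axes add yaw and pitch to the Camera.
; Left mouse press runs LocationDetect, which predicts a projectile arc from the camera and stores hits on near-horizontal WorldStatic surfaces.
; Release moves Scene to the stored X/Y, keeping its height; CanTeleport is never cleared, so a failed aim reuses the last valid target.
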(event EventBeginPlay)

(event Collision|EventActorBeginOverlap
  (params (OtherActor :type Actor%20Object%20Reference)))

(event EventTick
  (params (DeltaSeconds :type Float%20%28single-precision%29)))

(event Input|AxisEvents|InputAxisTurn
  (params (AxisValue :type Float%20%28single-precision%29))
  (Transformation|AddRelativeRotation (Variables|Default|GetCamera) (Math|Rotator|MakeRotator 0.0 0.0 AxisValue) false false))

(event Input|AxisEvents|InputAxisLookUp
  (params (AxisValue :type Float%20%28single-precision%29))
  (Transformation|AddRelativeRotation (Variables|Default|GetCamera) (Math|Rotator|MakeRotator 0.0 AxisValue 0.0) false false))

(event Input|MouseEvents|LeftMouseButton
  (params (Key :type Key%20Structure :default "AnyKey"))
  (bind _scene (Variables|Default|GetScene))
  (bind _camera (Variables|Default|GetCamera))
  (bind _telelocation (Variables|Default|GetTeleLocation))
  (bind (_x _y) (Math|Vector|BreakVector _telelocation))
  (:Pressed
    (Teleport|LocationDetect (Transformation|GetWorldLocation _camera) (Math|Vector|GetForwardVector _camera)))
  (:Released
    (if (Variables|Default|GetCanTeleport)
      (Transformation|SetWorldLocation _scene (Math|Vector|MakeVector _x _y (.Z (Math|Vector|BreakVector (Transformation|GetWorldLocation _scene)))) false true))))

(fn ConstructionScript)

(fn LocationDetect
  (params (CtrlLocation :type Vector) (CtrlForward :type Vector))
  (bind _outhit (Class|GameplayStatics|BlueprintPredictProjectilePathbyObjectType CtrlLocation (* CtrlForward 1e+03) true 0.0 (Utilities|Array|MakeArray "ObjectTypeQuery1") false 0 "None"))
  (if (> (Math|Vector|DotProduct (.Normal (Collision|BreakHitResult _outhit)) "0, 0,1.000000") 0.9)
    (Variables|Default|SetCanTeleport (> (Math|Vector|DotProduct (.Normal (Collision|BreakHitResult _outhit)) "0, 0,1.000000") 0.9))
    (Variables|Default|SetTeleLocation (.Location (Collision|BreakHitResult _outhit)))))